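; BP_Granade_40 is a HeavyGun grenade actor that explodes on a fixed one-second timer after spawning.
; BeginPlay yaws the static mesh by -90 degrees, waits, then calls Explode.
; Explode spawns a particle burst, applies full radial damage without falloff, adds radial force to its own mesh only, and destroys the actor.
; Debug spheres visualize the separate damage and force radii.
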(event Custom|Explode
  (bind _returnvalue (Transformation|GetActorLocation))
  (Effects|SpawnEmitteratLocation "/Game/WeaponEffects/Explosion/P_Explosion.P_Explosion" _returnvalue "0, 0, 0" "1.000000,1.000000,1.000000" true "AutoRelease")
  (Game|Damage|ApplyRadialDamage 1e+02 _returnvalue (Variables|Default|GetDamageRadius) 0 0 self (Game|GetInstigatorController) true "ECC_Visibility")
  (Physics|AddRadialForce (Variables|Default|GetStaticMesh) _returnvalue (Variables|Default|GetForceRadius) 1e+02 "RIF_Constant" true)
  (Actor|DestroyActor)
  (Rendering|Debug|DrawDebugSphere _returnvalue (Variables|Default|GetDamageRadius) 12 "(R=0.014659,G=1.000000,B=0.057785,A=1.000000)" 1.5 1.5)
  (Rendering|Debug|DrawDebugSphere _returnvalue (Variables|Default|GetForceRadius) 12 "(R=1.000000,G=0.709827,B=0.168136,A=1.000000)" 1.5 1.5))

(event EventBeginPlay
  (bind _staticmesh (Variables|Default|GetStaticMesh))
  (bind _returnvalue (Transformation|GetWorldRotation _staticmesh))
  (Transformation|SetWorldRotation _staticmesh (Math|Rotator|MakeRotator (.roll _returnvalue) (.pitch _returnvalue) (+ (.yaw _returnvalue) -9e+01)) false false)
  (Utilities|FlowControl|Delay 1.0)
  (CallFunction|Explode))

(fn ConstructionScript)